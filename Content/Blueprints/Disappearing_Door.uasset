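; A door actor that sinks far below its starting position once enough buttons have been activated.
; Each Triggered_Box call increments a counter, and reaching ButtonsNeeded plays a sliding sound and sets a target deep beneath the initial location.
; Tick continuously eases the Z position toward that target with a slow FInterpTo, keeping X and Y fixed.
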(event Custom|Triggered_Box
  (Math|Integer|IncrementInt (Variables|Default|GetButtonsActivated)
    (:%20%20
      (if (>= (Variables|Default|GetButtonsActivated) (Variables|Default|GetButtonsNeeded))
        (Audio|PlaySound2D "/Game/Sounds/zapsplat_science_fiction_door_slide_open_just_motor_sound_44437.zapsplat_science_fiction_door_slide_open_just_motor_sound_44437" 1.0 1.0 0.0 0 0)
        (Variables|Default|SetFinalPos (+ (Variables|Default|GetInitialPos) "0.000000,0.000000,-10000.000000"))))))

(event EventBeginPlay
  (Variables|Default|SetButtonsActivated 0)
  (bind _output_get (Variables|Default|SetInitialPos (Transformation|GetActorLocation)))
  (bind _output_get_2 (Variables|Default|SetCurrentPos _output_get))
  (Variables|Default|SetFinalPos _output_get_2))

(event EventTick
  (params (DeltaSeconds :type Float%20%28single-precision%29))
  (bind _initialpos (Variables|Default|GetInitialPos))
  (bind _output_get (Variables|Default|SetCurrentPos (Math|Vector|MakeVector (.x _initialpos) (.y _initialpos) (Math|Interpolation|FInterpTo (.z (Variables|Default|GetCurrentPos)) (.z (Variables|Default|GetFinalPos)) DeltaSeconds 0.05))))
  (Transformation|SetActorLocation _output_get false false))

(fn ConstructionScript)