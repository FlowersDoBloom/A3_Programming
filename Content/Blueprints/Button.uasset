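; Button actor that sends a referenced Platform moving through a cycle of preset positions.
; ButtonPressed briefly flashes the button mesh gray, then after a short delay advances the position index, wrapping it at three.
; Tick converts the current local position to world space and nudges the Platform toward it at MoveSpeed along a normalized direction, with no sweep or arrival check.
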(event Custom|Button%20Pressed
  (Rendering|Material|SetMaterial (Variables|Default|Geter) 0 "/Game/Textures/GRAY.GRAY")
  (Utilities|FlowControl|Delay 0.2)
  (Rendering|Material|SetMaterial (Variables|Default|Geter) 0 "/Game/StarterContent/Materials/M_Basic_Wall.M_Basic_Wall")
  (bind _result (Math|Integer|IncrementInt (Variables|Default|GetPositionNumber))
    (:%20%20
      (if (== _result 3)
        (Variables|Default|SetPositionNumber 0)))))

(event EventBeginPlay)

(event Collision|EventActorBeginOverlap
  (params (OtherActor :type Actor%20Object%20Reference)))

(event EventTick
  (params (DeltaSeconds :type Float%20%28single-precision%29))
  (bind _platform (Variables|Default|GetPlatform))
  (Transformation|AddActorWorldOffset _platform (* (Math|Vector|Normalize (- (Math|Transform|TransformLocation (Transformation|GetActorTransform) (Utilities|Array|Get(acopy) (Variables|Default|GetPositions) (Variables|Default|GetPositionNumber))) (Transformation|GetWorldLocation (Variables|/Script/Engine.StaticMeshActor|GetStaticMeshComponent _platform)))) (Variables|Default|GetMoveSpeed) DeltaSeconds)))

(fn ConstructionScript)